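; GM_WaveGame is a game mode that spawns an AI-controlled alien enemy when play begins.
; BeginPlay scans all PlayerStarts by tag, collecting EnemySpawn points in EnemyStart, while PlayerSpawn points are re-added to the full PlayerStartBase list.
; SpawnEnemy creates one Alien_Base at a random enemy start, then spawns an AIC_Alien controller to possess it.
; No repeat wave logic exists, and the empty-array check before spawning is disconnected.
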(event Custom|SpawnEnemy
  (bind _returnvalue (Game|SpawnActorfromClass "/Game/_Core/IA/Enemies/Alien/Alien_Base.Alien_Base_C" (Math|Transform|MakeTransform (Transformation|GetActorLocation (Utilities|Array|Get(acopy) (Variables|Default|GetEnemyStart) (Math|Random|RandomInteger (Utilities|Array|Length (Variables|Default|GetEnemyStart))))) "0, 0, 0" "1.000000,1.000000,1.000000") "AdjustIfPossibleButAlwaysSpawn" "MultiplyWithRoot" 0 0))
  (bind _output_get (Variables|Default|SetEnemy _returnvalue))
  (bind _returnvalue_2 (Game|SpawnActorfromClass "/Game/_Core/IA/Enemies/Alien/AIC_Alien.AIC_Alien_C" (Math|Transform|MakeTransform "0, 0, 0") "AlwaysSpawn" "MultiplyWithRoot" 0 0))
  (Pawn|Possess _returnvalue_2 _output_get))

(event EventBeginPlay
  (bind _outactors (Actor|GetAllActorsOfClass "/Script/Engine.PlayerStart"))
  (bind _output_get (Variables|Default|SetPlayerStartBase _outactors))
  (for _array_element _output_get
    (if (== (Variables|/Script/Engine.PlayerStart|GetPlayerStartTag _array_element) "EnemySpawn")
      (Utilities|Array|AddUnique (Variables|Default|GetEnemyStart) _array_element)
      (elif (== (Variables|/Script/Engine.PlayerStart|GetPlayerStartTag _array_element) "PlayerSpawn")
        (Utilities|Array|AddUnique (Variables|Default|GetPlayerStartBase) _array_element))))
  (CallFunction|SpawnEnemy))

(event EventTick
  (params (DeltaSeconds :type Float%20%28single-precision%29)))

(fn ConstructionScript)