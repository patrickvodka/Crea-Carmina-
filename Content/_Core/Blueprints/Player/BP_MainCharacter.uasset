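; Player character Blueprint with state-driven movement speed and helpers for measuring walls, apparently for vaulting or climbing.
; SetCharacterState records the previous state and updates max walk speed for walk, sprint, crouch, prone or dead.
; Line traces offset along the wall normal find wall height and thickness.
; DisableInput and EnableInput toggle movement mode and collision rather than input; EnableInput restores only capsule collision, not the mesh's.
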(fn ConstructionScript)

(fn SetCharacterState
  (params (NewState :type ECharacterState%20Enum :default "NewEnumerator0"))
  (if (Utilities|Enum|NotEqual(Enum) NewState (Variables|Default|GetCurrentCharacterState))
    (Variables|Default|SetPrevisouCharacterState (Variables|Default|GetCurrentCharacterState))
    (Variables|Default|SetCurrentCharacterState NewState)
    (CallFunction|UpdateSpeed)))

(fn UpdateSpeed
  (Variables|/Script/Engine.CharacterMovementComponent|SetMaxWalkSpeed (Variables|Character|GetCharacterMovement) (Utilities|Select :Index (Variables|Default|GetCurrentCharacterState) :NewEnumerator0 2e+02 :NewEnumerator1 4e+02 :NewEnumerator2 8e+01 :NewEnumerator3 5e+01 :NewEnumerator4 0.0)))

(fn CalculateWallHeight
  (bind (_returnvalue _returnvalue2 _draw_debug_type _object_types) (|CalculateHeightForLineTrace -1e+01))
  (bind _outhit (Collision|LineTraceForObjects _returnvalue2 _returnvalue _object_types false 0 _draw_debug_type))
  (Variables|Default|SetWall%20Height1 (.Location (Collision|BreakHitResult _outhit)))
  (return))

(fn CalculateWallThickness
  (bind (_returnvalue _returnvalue2 _draw_debug_type _object_types) (|CalculatethicknessForLineTrace_2 -7e+01))
  (bind (_outhit _returnvalue_2) (Collision|LineTraceForObjects _returnvalue2 _returnvalue _object_types false 0 _draw_debug_type))
  (return _returnvalue_2 (.Location (Collision|BreakHitResult _outhit))))

(fn DisableInput
  (Pawn|Components|CharacterMovement|SetMovementMode (Variables|Character|GetCharacterMovement) "MOVE_Flying" 0)
  (Collision|SetCollisionEnabled (Variables|Collision|GetCapsuleComponent) "NoCollision")
  (Collision|SetCollisionEnabled (Variables|Character|GetMesh) "NoCollision"))

(fn EnableInput
  (Pawn|Components|CharacterMovement|SetMovementMode (Variables|Character|GetCharacterMovement) "MOVE_Falling" 0)
  (Collision|SetCollisionEnabled (Variables|Collision|GetCapsuleComponent) "QueryAndPhysics"))