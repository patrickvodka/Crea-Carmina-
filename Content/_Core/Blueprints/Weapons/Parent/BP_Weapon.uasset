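; BP_Weapon is the parent weapon Actor, configured from a DAWeapon data asset.
; On BeginPlay, the See event validates the asset and mesh, sets the static mesh, and caches damage, range, fire-mode and bullet-count settings.
; Multi_FireFX spawns the asset's muzzle effect attached to the mesh's Muzzle socket.
; It contains no firing or damage logic, and its NewFunction mesh setter is not called here.
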(event Custom|See
  (bind _da_weapon (Variables|WeaponData|GetDA_Weapon)
    (:then
      (bind _staticmesh (Variables|Default|GetStaticMesh)
        (:then
          (bind _returnvalue (Components|StaticMesh|SetStaticMesh _staticmesh (Variables|/Game/_Core/FrameWorks/Data/PDA/PDA_Weapon.PDA_Weapon_C|GetWeapon_Mesh _da_weapon)))
          (if _returnvalue
            _
            (else
              _))
          (Variables|WeaponData|SetMaxDamage (Variables|/Game/_Core/FrameWorks/Data/PDA/PDA_Weapon.PDA_Weapon_C|GetDamageMax/Bullet (Variables|WeaponData|GetDA_Weapon)))
          (Variables|WeaponData|SetDamageModifier (Variables|/Game/_Core/FrameWorks/Data/PDA/PDA_Weapon.PDA_Weapon_C|GetDamageFallOff%20%20%20 (Variables|WeaponData|GetDA_Weapon)))
          (Variables|WeaponData|SetMaxDistance (Variables|/Game/_Core/FrameWorks/Data/PDA/PDA_Weapon.PDA_Weapon_C|GetMaxDistance (Variables|WeaponData|GetDA_Weapon)))
          (Variables|WeaponData|SetAutomaticFire (Variables|/Game/_Core/FrameWorks/Data/PDA/PDA_Weapon.PDA_Weapon_C|GetisAutomaticFire (Variables|WeaponData|GetDA_Weapon)))
          (Variables|WeaponData|SetSpreadFire (Variables|/Game/_Core/FrameWorks/Data/PDA/PDA_Weapon.PDA_Weapon_C|GetisSpreadFire (Variables|WeaponData|GetDA_Weapon)))
          (Variables|WeaponData|SetMaxNbrOfBullets (Variables|/Game/_Core/FrameWorks/Data/PDA/PDA_Weapon.PDA_Weapon_C|GetNumberOfBulletsMax (Variables|WeaponData|GetDA_Weapon))))
        (:else)))
    (:else)))

(event Custom|Multi_FireFX
  (Niagara|SpawnSystemAttached (Variables|/Game/_Core/FrameWorks/Data/PDA/PDA_Weapon.PDA_Weapon_C|GetMuzzleFX (Variables|WeaponData|GetDA_Weapon)) (Variables|Default|GetStaticMesh) "Muzzle" "0, 0, 0" "0, 0, 0" "KeepRelativeOffset" true))

(event EventBeginPlay
  (CallFunction|See))

(event Collision|EventActorBeginOverlap
  (params (OtherActor :type Actor%20Object%20Reference)))

(event EventTick
  (params (DeltaSeconds :type Float%20%28single-precision%29)))

(fn ConstructionScript)

(fn NewFunction
  (params (self2 :type Static%20Mesh%20Component%20Object%20Reference) (self3 :type PDA%20Weapon%20Object%20Reference))
  (Components|StaticMesh|SetStaticMesh self2 (Variables|/Game/_Core/FrameWorks/Data/PDA/PDA_Weapon.PDA_Weapon_C|GetWeapon_Mesh self3)))