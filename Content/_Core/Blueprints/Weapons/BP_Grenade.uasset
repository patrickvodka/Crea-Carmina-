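; BP_Grenade is a thrown grenade actor that explodes on a timed fuse and damages nearby targets.
; Tick waits until the throwing character supplies a non-zero LinearVelocity, then a server event launches the physics sphere once and starts the fuse delay.
; On detonation it damages overlap-tracked actors that carry the required tag and an AC_HealthManager component.
; A multicast then plays the Niagara effect, hides the sphere and destroys the actor.
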(event OnComponentBeginOverlap(Spherecol)
  (params (OverlappedComponent :type Primitive%20Component%20Object%20Reference) (OtherActor :type Actor%20Object%20Reference) (OtherComp :type Primitive%20Component%20Object%20Reference) (OtherBodyIndex :type Integer) (bFromSweep :type Boolean) (SweepResult :type Hit%20Result%20Structure%20%28by%20ref%29))
  ;[1 1 1] Actor in & out
  (Utilities|Array|AddUnique (Variables|Default|GetHittedActors) OtherActor))

(event OnComponentEndOverlap(Spherecol)
  (params (OverlappedComponent :type Primitive%20Component%20Object%20Reference) (OtherActor :type Actor%20Object%20Reference) (OtherComp :type Primitive%20Component%20Object%20Reference) (OtherBodyIndex :type Integer))
  ;[1 1 1] Actor in & out
  (Utilities|Array|RemoveItem (Variables|Default|GetHittedActors) OtherActor))

(event Custom|S_StartExplosion
  ;[1 1 1] Server code  to apply damage after a timing
  (Physics|SetPhysicsLinearVelocity (Variables|Default|GetSphere) (* (Variables|Default|GetLinearVelocity) (Variables|Default|GetSpeed)) false "None")
  (Utilities|FlowControl|Delay 4.0)
  (for _array_element (Variables|Default|GetHittedActors)
    (if (Actor|ActorHasTag _array_element (Variables|Default|GetTagOfNeededObjToHit))
      (Utilities|IsValid (Actor|GetComponentbyClass _array_element "/Game/_Core/Blueprints/AC/AC_HealthManager.AC_HealthManager_C")
        (:Is%20Valid
          (Game|Damage|ApplyDamage _array_element 1e+02 0 0)))))
  (CallFunction|MStartExplosion (Transformation|GetWorldLocation (Variables|Default|GetSphere))))

(event Custom|M_StartExplosion
  (params (SpawnVector :type Vector))
  ;[1 1 1] Multicast for the niagara & destroy
  (Transformation|SetRelativeLocation (Variables|Default|GetNiagara) (Math|Transform|InverseTransformLocation (Transformation|GetActorTransform) SpawnVector) false false)
  (Components|Activation|Activate (Variables|Default|GetNiagara) false)
  (Development|SetHiddeninGame (Variables|Default|GetSphere) true true)
  (Utilities|FlowControl|Delay 2.5)
  (Utilities|IsValid self
    (:Is%20Valid
      (Actor|DestroyActor))))

(event EventTick
  (params (DeltaSeconds :type Float%20%28single-precision%29))
  ;[1 1 1] We Wait until linear velocity is given by the third character
  ;;[1 1 1] ChangedTickSettings
  (if (not (Variables|Default|GetisExploded))
    (if (Utilities|Operators|NotEqual(!=) :A (Variables|Default|GetLinearVelocity))
      (Utilities|FlowControl|DoOnce false
        (:Completed
          (Variables|Default|SetisExploded true)
          (CallFunction|SStartExplosion))))))

(fn ConstructionScript)