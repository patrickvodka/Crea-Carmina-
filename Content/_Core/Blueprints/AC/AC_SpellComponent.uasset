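; Spell component that spawns spell actors in the world relative to its owner.
; EquipSpell casts immediately when CanCast is set, without using or storing the passed spell data.
; ExecuteSpell always spawns BP_SpellWall 500 units along the owner's forward vector.
; The Spell.Area tag check on EquippedSpell and the BP_SpellArea spawn at the owner's location are present but never run.
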(event Custom|EquipSpell
  (params (SpellData :type S%20Spell%20Data%20Structure))
  (bind _cancastspell (CallFunction|CastSpell))
  (if _cancastspell
    (CallFunction|ExecuteSpell)))

(event Custom|ExecuteSpell
  (bind _returnvalue (Components|GetOwner))
  (if true
    (Game|SpawnActorfromClass "/Game/_Core/Blueprints/Magic/Spells/BP_SpellWall.BP_SpellWall_C" (Math|Transform|MakeTransform (+ (Transformation|GetActorLocation _returnvalue) (* (Transformation|GetActorForwardVector _returnvalue) 500)) "0, 0, 0" "1.000000,1.000000,1.000000") "Undefined" "MultiplyWithRoot" 0 0)))

(event EventBeginPlay)

(event EventTick
  (params (DeltaSeconds :type Float%20%28single-precision%29)))

(fn CastSpell
  (if (Variables|Default|GetCanCast)
    (return true)
    (else
      (return false))))