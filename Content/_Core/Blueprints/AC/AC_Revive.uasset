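; Actor component that handles the downed, bleedout and revive cycle for its owning actor, tracked through LifeState.
; An Alive owner becomes Downed, starting a one-shot bleedout timer and a looping sphere-overlap check for other BP_ThirdPersonCharacter pawns.
; Any character in range revives it immediately, with no hold time, while timer expiry sets it Dead.
; Dispatchers announce each transition, and debug spheres and prints are still active.
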(event Custom|RevivePlayerCheck
  (bind _returnvalue (Components|GetOwner))
  (bind _reviverange (Variables|Default|GetReviveRange))
  (bind _returnvalue_2 (Transformation|GetActorLocation _returnvalue))
  ;[1 0.6256 0] Revive   & Bleedout
  ;;[0.7894 1 0.05415] Player Revive check
  (Rendering|Debug|DrawDebugSphere _returnvalue_2 _reviverange 12 "(R=0.000000,G=0.000000,B=0.000000,A=1.000000)" 0.1 1e+01)
  (bind (_outactors _returnvalue_3) (Collision|SphereOverlapActors _returnvalue_2 _reviverange (Utilities|Array|MakeArray "ObjectTypeQuery3") "/Game/ThirdPerson/Blueprints/BP_ThirdPersonCharacter.BP_ThirdPersonCharacter_C" (Utilities|Array|MakeArray _returnvalue)))
  (if _returnvalue_3
    (for _array_element _outactors
      (Development|PrintString (Utilities|GetDisplayName _array_element)))
    (Utilities|Time|ClearandInvalidateTimerbyHandle (Variables|Default|GetreviveTimer))
    (Utilities|Time|ClearandInvalidateTimerbyHandle (Variables|Default|GetBleedoutTimer))
    (Variables|Default|SetLifeState "NewEnumerator8")
    (Default|CallOnReviveCompleted)))

(event Custom|CanBeDownedCheck
  (switch Utilities|FlowControl|Switch|SwitchonE_PlayerLifeState (Variables|Default|GetLifeState)
    (:NewEnumerator8
      (CallFunction|SEnterDown))))

(event Custom|maxBleedOutTimer
  ;[1 0.6256 0] Revive   & Bleedout
  (bind _returnvalue (Utilities|Time|SetTimerbyEvent (delegate Custom|BleedoutEndEvent) (Variables|Default|GetReviveDuration)))
  (Variables|Default|SetBleedoutTimer _returnvalue))

(event Custom|BleedoutEndEvent
  ;[1 0.6256 0] Revive   & Bleedout
  ;;[1 0.1394 0] didn't revive in time
  (Development|PrintString (Utilities|String|Append "bleededOut" "  :   " (Utilities|GetDisplayName (Components|GetOwner))))
  (Utilities|Time|ClearandInvalidateTimerbyHandle (Variables|Default|GetreviveTimer))
  (Utilities|Time|ClearandInvalidateTimerbyHandle (Variables|Default|GetBleedoutTimer))
  (Variables|Default|SetLifeState "NewEnumerator5")
  (Default|CallOnBleededOut (Components|GetOwner)))

(event Custom|S_EnterDown
  (Variables|Default|SetLifeState "NewEnumerator7")
  (Default|CallOnDowned (Components|GetOwner))
  (CallFunction|StartBleedout))

(event Custom|StartBleedout
  ;[1 0.6256 0] Revive   & Bleedout
  ;;[1 0 0] 1.0  - Bleedout
  (CallFunction|MaxBleedOutTimer)
  (bind _returnvalue (Utilities|Time|SetTimerbyEvent (delegate Custom|RevivePlayerCheck) 0.1 true true))
  (Variables|Default|SetreviveTimer _returnvalue))