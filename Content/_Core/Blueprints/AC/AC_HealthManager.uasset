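; AC_HealthManager is a component that tracks its owner's health, set to MaxHealth at BeginPlay through S_BeginPlay.
; S_TakeDamage and S_Heal feed functions that clamp CurrentHealth between zero and max, then fire health-changed and damaged or healed dispatchers.
; Damage reaching zero also fires OnPreDeath, leaving death handling outside these graphs.
; Heal's ShieldAmount is unused, overheal is always reported false, and the OnRep function is empty.
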(event Custom|S_TakeDamage
  (params (DamageType :type S%20Damage%20Type%20Structure))
  ;[1 0 0] Damage
  (CallFunction|TakeDamageFonct DamageType))

(event Custom|S_BeginPlay
  ;[1 0.3597 0] Setup at start the maxHealth
  (Variables|Default|SetCurrentHealth (Variables|Default|GetMaxHealth)))

(event Custom|S_Heal
  (params (HealAmount :type Float%20%28double-precision%29) (ShieldAmount :type Float%20%28double-precision%29))
  ;[0 1 0.02558] Heal
  (CallFunction|HealFonct HealAmount))

(event EventBeginPlay
  ;[1 0.3597 0] Setup at start the maxHealth
  (CallFunction|SBeginPlay))

(fn OnRepCurrentHealthServ)

(fn HealFonct
  (params (HealNbr :type Float%20%28double-precision%29))
  (LocalVariables|SetHealthbeforeHeal (Variables|Default|GetCurrentHealth))
  (bind _output_get (Variables|Default|SetCurrentHealth (Math|Float|Clamp(Float) (+ (Variables|Default|GetCurrentHealth) HealNbr) 0.0 (Variables|Default|GetMaxHealth))))
  (Default|CallOnHealthChanged false (LocalVariables|GetHealthbeforeHeal) _output_get)
  (Default|CallOnHealed HealNbr false 0.0)
  (return))

(fn TakeDamageFonct
  (params (DamageType :type S%20Damage%20Type%20Structure))
  (LocalVariables|SetDamageTypeLocal DamageType)
  (LocalVariables|SetHealthBeforeDamage (Variables|Default|GetCurrentHealth))
  (Variables|Default|SetCurrentHealth (Math|Float|Clamp(Float) (- (Variables|Default|GetCurrentHealth) (.Damage (Utilities|Struct|BreakS_DamageType (LocalVariables|GetDamageTypeLocal)))) 0.0 (Variables|Default|GetMaxHealth)))
  (Default|CallOnHealthChanged true (LocalVariables|GetHealthBeforeDamage) (Variables|Default|GetCurrentHealth))
  (Default|CallOnDamageTaken (LocalVariables|GetDamageTypeLocal))
  (if (<= (Variables|Default|GetCurrentHealth) 0.0)
    (Default|CallOnPreDeath)
    (return)
    (else
      (return))))