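; Magic crafting table that holds gems in a cell grid, with shape recognition apparently meant for spell building.
; Gems are placed or removed by index, and occupied cells normalize into a bounding-box boolean pattern for matching against data-asset shapes.
; FindShapeInCells instead scans anchor cells for each shape but returns no result.
; Work in progress: BuildSpell is empty, DetectAllShapes is unfinished, and FindMatchingShape compares only dimensions because its cell comparison is unwired.
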(event Custom|BuildSpell)

(event EventBeginPlay
  (CallFunction|InitializeGrid false))

(fn ConstructionScript)

(fn InitializeGrid
  (params (ShouldClearIt :type Boolean))
  (if ShouldClearIt
    (Utilities|Array|Clear (Variables|Default|GetGridCells)))
  (for _index (range 0 24)
    (Utilities|Array|Add (Variables|Default|GetGridCells) (Utilities|Struct|MakeS_CraftCell)))
  (return))

(fn PlaceGem
  (params (CellIndex :type Integer) (Gem :type PDA%20Gem%20Object%20Reference))
  (Utilities|IsValid Gem
    (:Is%20Valid
      (if (and (>= CellIndex 0) (< CellIndex (Utilities|Array|Length (Variables|Default|GetGridCells))))
        (Utilities|Array|SetArrayElem (Variables|Default|GetGridCells) CellIndex (Utilities|Struct|MakeS_CraftCell Gem))
        (return true)
        (else
          (return false))))
    (:Is%20Not%20Valid
      (return false))))

(fn RemoveGem
  (params (CellIndex :type Integer))
  (if (and (>= CellIndex 0) (< CellIndex (Utilities|Array|Length (Variables|Default|GetGridCells))))
    (Utilities|Array|SetArrayElem (Variables|Default|GetGridCells) CellIndex (Utilities|Struct|MakeS_CraftCell 0))
    (return true)
    (else
      (return false))))

(fn GetOccupiedCells
  (for _index (range 0 (- (Utilities|Array|Length (Variables|Default|GetGridCells)) 1))
    (Utilities|IsValid (Utilities|Struct|BreakS_CraftCell (Utilities|Array|Get(acopy) (Variables|Default|GetGridCells) _index))
      (:Is%20Valid
        (Utilities|Array|Add (LocalVariables|GetLocalOccupiedCells) _index))))
  (return (LocalVariables|GetLocalOccupiedCells)))

(fn NormalizePattern
  (params (occupîedCells :type Array%20of%20Integers))
  (for _array_element occupîedCells
    (LocalVariables|SetMinX (Math|Integer|Min(Integer) (LocalVariables|GetMinX) (Math|Integer|%(Integer) _array_element (Variables|Default|GetGridWidth))))
    (LocalVariables|SetMaxX (Math|Integer|Max(Integer) (LocalVariables|GetMaxX) (Math|Integer|%(Integer) _array_element (Variables|Default|GetGridWidth))))
    (LocalVariables|SetMinY (Math|Integer|Min(Integer) (LocalVariables|GetMinY) (/ _array_element (Variables|Default|GetGridWidth))))
    (LocalVariables|SetMaxY (Math|Integer|Max(Integer) (LocalVariables|GetMaxY) (/ _array_element (Variables|Default|GetGridWidth)))))
  (bind _output_get (LocalVariables|SetPatternWidth (+ (- (LocalVariables|GetMaxX) (LocalVariables|GetMinX)) 1)))
  (bind _output_get_2 (LocalVariables|SetPatternHeight (+ (- (LocalVariables|GetMaxY) (LocalVariables|GetMinY)) 1)))
  ;[0 0 0] Set All array to false
  (for _index (range 0 (- (* _output_get_2 _output_get) 1))
    (Utilities|Array|Add (LocalVariables|GetPatternCells) false))
  (for _array_element_2 occupîedCells
    (Utilities|Array|SetArrayElem (LocalVariables|GetPatternCells) (+ (* (- (/ _array_element_2 (Variables|Default|GetGridWidth)) (LocalVariables|GetMinY)) (LocalVariables|GetPatternWidth)) (- (Math|Integer|%(Integer) _array_element_2 (Variables|Default|GetGridWidth)) (LocalVariables|GetMinX))) true))
  (return (Utilities|Struct|MakeS_ShapePattern (LocalVariables|GetPatternWidth) (LocalVariables|GetPatternHeight) (LocalVariables|GetPatternCells))))

(fn FindMatchingShape
  (params (Pattern :type S%20Shape%20Pattern%20Structure))
  (bind (_width _height _cells) (Utilities|Struct|BreakS_ShapePattern Pattern))
  (bind _availableshapes (Variables|Default|GetAvailableShapes))
  (Utilities|IsValid _availableshapes
    (:Is%20Valid
      (for _array_element (Variables|/Game/_Core/FrameWorks/Data/PDA/PDA_MagicCraftConfig.PDA_MagicCraftConfig_C|GetAvailableShapes _availableshapes)
        (Utilities|IsValid _array_element
          (:Is%20Valid
            (if (Math|Boolean|ANDBoolean (== _width (.width (Variables|/Game/_Core/FrameWorks/Data/PDA/PDA_Shape.PDA_Shape_C|GetPattern _array_element))) (== (Utilities|Array|Length _cells) (Utilities|Array|Length (.cells (Variables|/Game/_Core/FrameWorks/Data/PDA/PDA_Shape.PDA_Shape_C|GetPattern _array_element)))) (== _height (.height (Variables|/Game/_Core/FrameWorks/Data/PDA/PDA_Shape.PDA_Shape_C|GetPattern _array_element))))
              (LocalVariables|SetbPatternMatches true)
              (for _index (range 0 (- (Utilities|Array|Length (.cells (Variables|/Game/_Core/FrameWorks/Data/PDA/PDA_Shape.PDA_Shape_C|GetPattern _array_element))) 1))
                (if (not (LocalVariables|GetbPatternMatches))
                  (LocalVariables|SetbPatternMatches false)))
              (if (LocalVariables|GetbPatternMatches)
                (return _array_element)))))))
    (:Is%20Not%20Valid
      (Development|PrintString "DA_MagicCraftConfigMissing")))
  (return 0))

(fn DetectAllShapes
  (bind _occupiedcells (CallFunction|GetOccupiedCells))
  (LocalVariables|SetRemainingCells _occupiedcells))

(fn FindShapeinCells
  (params (CandidateCells :type Array%20of%20Integers))
  (bind _availableshapes (Variables|Default|GetAvailableShapes)
    (:then
      (for _array_element (Variables|/Game/_Core/FrameWorks/Data/PDA/PDA_MagicCraftConfig.PDA_MagicCraftConfig_C|GetAvailableShapes _availableshapes)
        (LocalVariables|SetRequiredCellCount 0)
        (bind _output_get (LocalVariables|SetCurrentPattern (Variables|/Game/_Core/FrameWorks/Data/PDA/PDA_Shape.PDA_Shape_C|GetPattern _array_element)))
        (for _array_element_2 (.Cells (Utilities|Struct|BreakS_ShapePattern _output_get))
          (if _array_element_2
            (Math|Integer|IncrementInt (LocalVariables|GetRequiredCellCount))))
        (if (>= (Utilities|Array|Length CandidateCells) (LocalVariables|GetRequiredCellCount))
          (for _array_element_3 CandidateCells
            (LocalVariables|SetAnchorY (/ _array_element_3 (Variables|Default|GetGridWidth)))
            (LocalVariables|SetAnchorX (Math|Integer|%(Integer) _array_element_3 (Variables|Default|GetGridWidth)))
            (Utilities|Array|Clear (LocalVariables|GetLocalMatchedCells))
            (LocalVariables|SetbMatch true)
            (for _index (range 0 (- (Utilities|Array|Length (.cells (LocalVariables|GetCurrentPattern))) 1))
              (if (Utilities|Array|Get(acopy) (.cells (LocalVariables|GetCurrentPattern)) _index)
                (LocalVariables|SetLocalX (Math|Integer|%(Integer) _index (.width (LocalVariables|GetCurrentPattern))))
                (bind _output_get_2 (LocalVariables|SetLocalY (/ _index (.width (LocalVariables|GetCurrentPattern)))))
                (bind _output_get_3 (LocalVariables|SetWorldY (+ _output_get_2 (LocalVariables|GetAnchorY))))
                (bind _output_get_4 (LocalVariables|SetWorldX (+ (LocalVariables|GetAnchorX) (LocalVariables|GetLocalX))))
                (bind _output_get_5 (LocalVariables|SetWorldIndex (+ _output_get_4 _output_get_3 (Variables|Default|GetGridWidth))))
                (if (Utilities|Array|ContainsItem CandidateCells _output_get_5)
                  (Utilities|Array|Add (LocalVariables|GetLocalMatchedCells) _output_get_5)
                  (else
                    (LocalVariables|SetbMatch false)))))))))
    (:else
      (return 0 0))))